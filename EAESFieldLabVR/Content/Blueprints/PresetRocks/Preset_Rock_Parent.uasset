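; Parent actor for preset rocks, holding each rock's identity, images, scale, discovery state and test results.
; BeginPlay loads the RockData struct, assigns a unique ID, caches the model transform and resets test states and results from the GameInstance test list.
; A lone RockID takes a new ID from GameInstance counters, while duplicates copy one from matching actors.
; SaveRockData repacks the struct, which InteractOpen returns.
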(event `self.ReceiveBeginPlay`
  (bind _rocktests (`self.RockTests`))
  ;[0 1 0] Event BeginPlay
  ;[1 1 1] Load Rock Data
  (`self.Load Rock Data`)
  ;[1 1 1] Assign Unique Rock ID
  (`self.Assign Rock Unique ID`)
  ;[1 1 1] Sets Rock Transform
  (set `self.Rock Transform` (`SceneComponent.K2_GetComponentToWorld` (`self.RockModel`)))
  ;[1 1 1] Initialize Rock Test Done for each Rock Test
  (bind _keys (`BlueprintMapLibrary.Map_Keys` (`self.RockTests`)))
  (for _array_element _keys
    (`BlueprintMapLibrary.Map_Add` (`self.RockTestDone`) _array_element))
  ;[1 1 1] Update Default Test Result
  (bind _aseaes_game_instance (cast `/Game/Misc/EAES-GameInstance` (`GameplayStatics.GetGameInstance`)))
  (for _array_element_2 (`/Game/Misc/EAES-GameInstance.RockTestList` _aseaes_game_instance)
    (switch `string` _array_element_2
      (:`Default`
        (`BlueprintMapLibrary.Map_Add` _rocktests _array_element_2 "N/A"))
      (:`Magnetic Test`
        (`BlueprintMapLibrary.Map_Add` _rocktests _array_element_2 "No"))
      (:`Acid Test`
        (`BlueprintMapLibrary.Map_Add` _rocktests _array_element_2 "No")))))

(event `Set Rock Scale`
  (params (`Scale Multiplier` :type "Float (double-precision)"))
  ;[0 1 1] Sets Rock Scale
  (bind _output_get (set `self.ScaleMultiplier` `Scale Multiplier`))
  (`SceneComponent.SetWorldScale3D` (`self.RockModel`) (* _output_get (.scale (`self.Rock Transform`)))))

(event `Save Rock Data`
  ;[0 1 1] Save Rock Data
  (set `self.RockData` (make `/Game/Misc/RockStruct` (`self.Rock ID`) (`self.Unique Rock ID`) (`self.Rock Display Name`) (`self.GetTransform`) (`self.ScaleMultiplier`) (`self.Rock Display Image`) (`self.Rock Microscopic Image`) (`self.isDiscovered?`) (`self.RockTests`) (`self.RockTestDone`) (`GameplayStatics.GetObjectClass` self))))

(event `Load Rock Data`
  (bind (_rockdata_rockid _rockdata_uniquerockid _rockdata_rockdisplayname _rockdata_rocktransform _rockdata_scalemultiplier _rockdata_rockdisplayimage _rockdata_thinsectionimage _rockdata_isdiscovered_ _rockdata_rocktests _rockdata_rocktestdone _rockdata_rockclass) (break `/Game/Misc/RockStruct` (`self.RockData`)))
  ;[0 1 1] Load Rock Data
  (set `self.Rock ID` _rockdata_rockid)
  (set `self.Unique Rock ID` _rockdata_uniquerockid)
  (set `self.Rock Display Name` _rockdata_rockdisplayname)
  (set `self.Rock Transform` _rockdata_rocktransform)
  (set `self.ScaleMultiplier` _rockdata_scalemultiplier)
  (set `self.Rock Display Image` _rockdata_rockdisplayimage)
  (set `self.Rock Microscopic Image` _rockdata_thinsectionimage)
  (set `self.isDiscovered?` _rockdata_isdiscovered_)
  (set `self.RockTests` _rockdata_rocktests)
  (set `self.RockTestDone` _rockdata_rocktestdone)
  (set `self.Rock Class` _rockdata_rockclass))

(event `Assign Rock Unique ID`
  ;[0 1 1] Assign Unique Rock ID
  (bind _aseaes_game_instance (cast `/Game/Misc/EAES-GameInstance` (`GameplayStatics.GetGameInstance`)))
  (set `self.Number of Instances` 0)
  (bind _outactors (`GameplayStatics.GetAllActorsOfClass` "Preset_Rock_Parent_C"))
  (for _array_element _outactors
    (if (== (`/Game/Blueprints/PresetRocks/Preset_Rock_Parent.Rock ID` _array_element) (`self.Rock ID`))
      (`/Engine/EditorBlueprintResources/StandardMacros.IncrementInt` (`self.Number of Instances`))))
  (switch `int` (`self.Number of Instances`)
    (:`Default`
      (bind _outactors_2 (`GameplayStatics.GetAllActorsOfClass` "Preset_Rock_Parent_C"))
      (for _array_element_2 _outactors_2
        (if (== (`/Game/Blueprints/PresetRocks/Preset_Rock_Parent.Rock ID` _array_element_2) (`self.Rock ID`))
          (set `self.Unique Rock ID` (`/Game/Blueprints/PresetRocks/Preset_Rock_Parent.Unique Rock ID` _array_element_2)))))
    (:`1`
      (bind _result (`/Engine/EditorBlueprintResources/StandardMacros.IncrementInt` (`/Game/Misc/EAES-GameInstance.Number of Unique Rocks` _aseaes_game_instance))
        (:`  `
          (set `self.Unique Rock ID` _result)
          (`/Engine/EditorBlueprintResources/StandardMacros.IncrementInt` (`/Game/Misc/EAES-GameInstance.Number of Unique Preset Rocks` _aseaes_game_instance)))))))

(fn `InteractOpen`
  (returns (ReturnRockData :type "/Game/Misc/RockStruct Structure"))
  (return (`self.RockData`)))

(fn `UserConstructionScript`)